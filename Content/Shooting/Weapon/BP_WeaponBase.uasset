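; Base weapon actor for the shooting game that a BP_ShootingCharacter can carry and fire, with each action reporting success as a boolean.
; AttachToActor snaps it to the character mesh's "weapon" socket and disables physics; DetachToActor calls detach on the passed Actor and re-enables weapon physics.
; DoShot only spawns a scaled-down explosion particle at the muzzle socket, with no projectile or damage.
; DoTrigger is a stub returning false.
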(event EventBeginPlay)

(event Collision|EventActorBeginOverlap
  (params (OtherActor :type Actor%20Object%20Reference)))

(event EventTick
  (params (DeltaSeconds :type Float%20%28single-precision%29)))

(fn ConstructionScript)

(fn AttachtoActor
  (params (Actor :type Character%20Object%20Reference))
  (bind _asbp_shooting_character (Utilities|Casting|CastToBP_ShootingCharacter Actor))
  (bind _returnvalue (Transformation|AttachComponentToComponent (Variables|/Script/Engine.Character|GetMesh _asbp_shooting_character) "weapon" "SnapToTarget" "SnapToTarget" "KeepWorld" true))
  (if _returnvalue
    (Physics|SetSimulatePhysics (Variables|Default|GetWeapon) false)
    (return true)
    (else
      (return false))))

(fn DetachtoActor
  (params (Actor :type Actor%20Object%20Reference))
  (Transformation|DetachFromActor Actor "KeepRelative" "KeepRelative" "KeepWorld")
  (Physics|SetSimulatePhysics (Variables|Default|GetWeapon) true)
  (return true))

(fn DoShot
  (bind _weapon (Variables|Default|GetWeapon))
  (bind _returnvalue (Transformation|GetSocketTransform _weapon "muzzle" "RTS_World"))
  (bind _returnvalue_2 (Effects|SpawnEmitteratLocation "/Game/StarterContent/Particles/P_Explosion.P_Explosion" (.location _returnvalue) (.rotation _returnvalue) "0.100000,0.100000,0.100000"))
  (Utilities|IsValid _returnvalue_2
    (:Is%20Valid
      (return true))
    (:Is%20Not%20Valid
      (return false))))

(fn DoTrigger
  (return false))