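; BP_NameTagComponet is a component that manages a name tag widget showing a name and current HP.
; On BeginPlay it creates the widget with a reference to itself and adds it to the viewport, then removes it on EndPlay.
; SetName and UpdateCurHpPercent pass the name and the current and max HP through to the widget.
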(event EventBeginPlay
  (bind _returnvalue (UserInterface|CreateWidget "/Game/Shooting/BluePrints/NameTagWidget.NameTagWidget_C" 0 self))
  (bind _output_get (Variables|Default|SetNameTagWidget _returnvalue))
  (UserInterface|Viewport|AddtoViewport _output_get 0))

(event EventEndPlay
  (params (EndPlayReason :type EEndPlayReason%20Enum :default "Destroyed"))
  (Widget|RemovefromParent (Variables|Default|GetNameTagWidget)))

(fn SetName
  (params (Name :type String))
  (Default|SetName (Variables|Default|GetNameTagWidget) Name))

(fn UpdateCurHpPercent
  (params (CurHp :type Float%20%28double-precision%29) (MaxHp :type Float%20%28double-precision%29))
  (Default|SetCurHpPercent (Variables|Default|GetNameTagWidget) CurHp MaxHp))